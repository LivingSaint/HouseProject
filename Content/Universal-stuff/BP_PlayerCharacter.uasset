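; BP_PlayerCharacter is the player character Blueprint, providing walking, look controls and an early-stage interact action.
; Axis inputs move the pawn along its forward and right vectors and feed controller yaw and pitch.
; Pressing E fires a Visibility line trace 1500 units along the camera's forward vector with persistent debug drawing.
; The trace result is not yet used, and a second trace node sits disconnected.
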(event `InputAxis|W_Forward/S_Back`
  (params (AxisValue :type "Float (single-precision)"))
  (`self.AddMovementInput` (`self.GetActorForwardVector`) AxisValue))

(event `InputAxis|A_Left/D_Right`
  (params (AxisValue :type "Float (single-precision)"))
  (`self.AddMovementInput` (`self.GetActorRightVector`) AxisValue))

(event `InputAxis|TurnOnXAxis`
  (params (AxisValue :type "Float (single-precision)"))
  (`self.AddControllerYawInput` AxisValue))

(event `InputAxis|TurnOnYAxis`
  (params (AxisValue :type "Float (single-precision)"))
  (`self.AddControllerPitchInput` AxisValue))

(event `InputAction|E_Interact`
  (params (Key :type "Key Structure"))
  (bind _camera (`self.Camera`))
  (bind _returnvalue (`SceneComponent.K2_GetComponentLocation` _camera))
  (:`Pressed`
    (bind _outhit (`KismetSystemLibrary.LineTraceSingle` :`Start` _returnvalue :`End` (+ _returnvalue (* (`KismetMathLibrary.GetForwardVector` (`SceneComponent.K2_GetComponentRotation` _camera)) 1500.0)) :`TraceChannel` "TraceTypeQuery1" :`DrawDebugType` "Persistent"))))

(fn `UserConstructionScript`)